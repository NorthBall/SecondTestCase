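; BP_Button is an interactible button that triggers the GA_SpawnTurtle ability through its own ability system component when activated.
; The ability is granted at ButtonLevel, and activation changes drive the Active parameter on a dynamic material tinted with ButtonColor.
; The construction script builds that material and copies spawn and destination locations from reference actors, binding to their location-change events to stay in sync until EndPlay.
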(event `self.ReceiveBeginPlay`
  (`self.OnActivationStateChanged`))

(event `OverrideMaterial`
  (bind _returnvalue (`KismetMaterialLibrary.CreateDynamicMaterialInstance` "/Game/SecondTestCase/Art/Materials/Button/M_Button.M_Button" "None" "Transient"))
  (`MaterialInstanceDynamic.SetVectorParameterValue` _returnvalue "ButtonColor" (`self.ButtonColor`))
  (`MaterialInstanceDynamic.SetScalarParameterValue` _returnvalue "Active" 0.0)
  (`PrimitiveComponent.SetMaterial` (`self.ButtonMesh`) 0 _returnvalue))

(event `self.InitASC`
  (`parent.InitASC`)
  (`STC_AbilitySystemComponent.AddAbilityByClass` (`self.ButtonASC`) "/Game/SecondTestCase/Abilities/Turtle/GA_SpawnTurtle.GA_SpawnTurtle_C" (`self.ButtonLevel`)))

(event `GetRefsLocation`
  (`|ExecutionSequence`
    (:`then_0`
      (bind _spawnlocationref (`self.SpawnLocationRef`)
        (:`then`
          (set `self.SpawnLocation` (`self.K2_GetActorLocation` _spawnlocationref))
          (`/Engine/EditorBlueprintResources/StandardMacros.DoOnce` false
            (:`Completed`
              (add `/Game/SecondTestCase/Utility/BP_LocationActor.OnLocationChanged` _spawnlocationref (delegate `OnSpawnLocationChanged`)))))
        (:`else`)))
    (:`then_1`
      (bind _destinationlocationref (`self.DestinationLocationRef`)
        (:`then`
          (set `self.DestinationLocation` (`self.K2_GetActorLocation` _destinationlocationref))
          (`/Engine/EditorBlueprintResources/StandardMacros.DoOnce` false
            (:`Completed`
              (add `/Game/SecondTestCase/Utility/BP_LocationActor.OnLocationChanged` _destinationlocationref (delegate `OnDestinationLocationChanged`)))))
        (:`else`)))))

(event `OnSpawnLocationChanged`
  (params (NewLocation :type "Vector Structure"))
  (set `self.SpawnLocation` NewLocation))

(event `OnDestinationLocationChanged`
  (params (NewLocation :type "Vector Structure"))
  (set `self.DestinationLocation` NewLocation))

(event `self.ReceiveEndPlay`
  (params (EndPlayReason :type "EEndPlayReason Enum" :default "Destroyed"))
  (`parent.ReceiveEndPlay` EndPlayReason)
  (`|ExecutionSequence`
    (:`then_0`
      (bind _spawnlocationref (`self.SpawnLocationRef`)
        (:`then`
          (remove `/Game/SecondTestCase/Utility/BP_LocationActor.OnLocationChanged` _spawnlocationref (`|CreateDelegate` :!event `OnSpawnLocationChanged`)))
        (:`else`)))
    (:`then_1`
      (bind _destinationlocationref (`self.DestinationLocationRef`)
        (:`then`
          (remove `/Game/SecondTestCase/Utility/BP_LocationActor.OnLocationChanged` _destinationlocationref (`|CreateDelegate` :!event `OnDestinationLocationChanged`)))
        (:`else`)))))

(fn `Activate`
  (returns (ReturnValue :type Boolean))
  (bind _returnvalue (`parent.Activate`))
  (if _returnvalue
    (`self.OnActivationStateChanged`)
    (`AbilitySystemComponent.TryActivateAbilityByClass` (`self.ButtonASC`) "/Game/SecondTestCase/Abilities/Turtle/GA_SpawnTurtle.GA_SpawnTurtle_C" true)
    (return true)
    (else
      (return false))))

(fn `Deactivate`
  (returns (ReturnValue :type Boolean))
  (bind _returnvalue (`parent.Deactivate`))
  (if _returnvalue
    (`self.OnActivationStateChanged`)
    (return true)
    (else
      (return false))))

(fn `OnActivationStateChanged`
  (bind _asmaterial_instance_dynamic (cast `MaterialInstanceDynamic` (`PrimitiveComponent.GetMaterial` (`self.ButtonMesh`) 0)))
  (`MaterialInstanceDynamic.SetScalarParameterValue` _asmaterial_instance_dynamic "Active" (select `bool` (`self.bIsActive`) :`true` 1.0 :!type "Float (single-precision)")))

(fn `UserConstructionScript`
  (`self.OverrideMaterial`)
  (`self.GetRefsLocation`))