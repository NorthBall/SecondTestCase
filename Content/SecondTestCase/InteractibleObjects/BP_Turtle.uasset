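; BP_Turtle is an AI-controlled turtle pawn that travels toward a destination location.
; InitBehaviorTree applies BB_Turtle to its AI controller and fills in the spawn location, destination and an inverse flag derived from TurtleBehavior; no tree is started here.
; SimpleMoveTurtle instead uses AI MoveTo directly and destroys the turtle whether the move succeeds or fails.
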(event `self.InitBehaviorTree`
  (bind _returnvalue (`AIBlueprintHelperLibrary.GetBlackboard` self))
  (`|ExecutionSequence`
    (:`then_0`
      (`AIController.UseBlackboard` (`AIBlueprintHelperLibrary.GetAIController` self) "/Game/SecondTestCase/AI/BB_Turtle.BB_Turtle"))
    (:`then_1`
      (`BlackboardComponent.SetValueAsVector` _returnvalue "SpawnLocation" (`self.SpawnLocation`))
      (`BlackboardComponent.SetValueAsVector` _returnvalue "DestinationLocation" (`self.DestinationLocation`))
      (`BlackboardComponent.SetValueAsBool` _returnvalue "bShouldInverse" (`|EnumEquality` (`self.TurtleBehavior`) "ETB_WithInverse")))))

(event `self.SimpleMoveTurtle`
  (`|AIMoveTo` (`AIBlueprintHelperLibrary.GetAIController` self) self (`self.DestinationLocation`) null 50.0
    (:`OnSuccess`
      _)
    (:`OnFail`
      _))
  (`self.K2_DestroyActor`))

(fn `UserConstructionScript`)