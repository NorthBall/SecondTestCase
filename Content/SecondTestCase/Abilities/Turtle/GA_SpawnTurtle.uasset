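; Gameplay ability that spawns a turtle using target data supplied by its owning interactible object through an interface.
; The data's origin and end point set the turtle's spawn and destination, and ability level selects straight, stopping or inverse movement behavior.
; A turtle gameplay cue lasts while the ability runs.
; The turtle's EndPlay ends the ability, which unbinds the event and sends the owner a deactivate message.
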(event `self.K2_ActivateAbility`
  (bind _targetdata (`self.GetOwnerTargetData`))
  (bind _returnvalue (`AbilitySystemBlueprintLibrary.GetTargetDataOrigin` _targetdata))
  (bind _returnvalue_2 (`|SpawnActorFromClass` "/Game/SecondTestCase/InteractibleObjects/BP_Turtle.BP_Turtle_C" _returnvalue "AdjustIfPossibleButAlwaysSpawn" "OverrideRootScale" null (.location _returnvalue) (`AbilitySystemBlueprintLibrary.GetTargetDataEndPoint` _targetdata) (select `int` (`self.GetAbilityLevel`) :`0` "ETB_StraightForward" :`1` "ETB_StraightForward" :`2` "ETB_WithStops" :`3` "ETB_WithInverse" :!type "ETB_TurtleBehavior Enum") null))
  (bind _output_get (set `self.ControlledTurtle` _returnvalue_2))
  (add `Actor.OnEndPlay` _output_get (delegate `OnTurtleEndPlay`))
  (`self.K2_AddGameplayCueWithParams` (struct :`TagName` "Cue.Turtle") (`AbilitySystemBlueprintLibrary.MakeGameplayCueParameters` 0.0 0.0 (struct) (struct) (struct) (struct) (struct) (0.0 0.0 0.0) (0.0 0.0 0.0) null (`self.ControlledTurtle`))))

(event `OnTurtleEndPlay`
  (params (Actor :type "Actor Object Reference") (EndPlayReason :type "EEndPlayReason Enum" :default "Destroyed"))
  (`self.K2_EndAbility`))

(event `self.K2_OnEndAbility`
  (params (bWasCancelled :type Boolean))
  (bind _returnvalue (`self.GetOwningActorFromActorInfo`))
  (`|ExecutionSequence`
    (:`then_0`
      (bind _controlledturtle (`self.ControlledTurtle`)
        (:`then`
          (remove `Actor.OnEndPlay` _controlledturtle (`|CreateDelegate` :!event `OnTurtleEndPlay`)))
        (:`else`)))
    (:`then_1`
      (`/Engine/EditorBlueprintResources/StandardMacros.IsValid` _returnvalue
        (:`Is Valid`
          (if (`KismetSystemLibrary.DoesImplementInterface` _returnvalue "/Script/SecondTestCase.STC_InteractibleObject")
            (message `STC_InteractibleObject.Deactivate` _returnvalue)))))))

(fn `GetOwnerTargetData`
  (returns (TargetData :type "GameplayAbilityTargetDataHandle Structure"))
  (bind _returnvalue (`self.GetOwningActorFromActorInfo`))
  (`/Engine/EditorBlueprintResources/StandardMacros.IsValid` _returnvalue
    (:`Is Valid`
      (if (`KismetSystemLibrary.DoesImplementInterface` _returnvalue "/Script/SecondTestCase.STC_InteractibleObject")
        (bind _returnvalue_2 (message `STC_InteractibleObject.GetTargetData` _returnvalue))
        (return _returnvalue_2)
        (else
          _)))
    (:`Is Not Valid`
      _))
  (return (make `GameplayAbilityTargetDataHandle`)))